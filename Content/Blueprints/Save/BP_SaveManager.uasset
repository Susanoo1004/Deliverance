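; BP_SaveManager is a save manager Blueprint that is currently inert: its events and save/load sync functions have empty bodies.
; Disconnected nodes sketch registering with SaveSystem for save callbacks and printing the slot name and saved location.
; An unwired SyncBeforeSave chain would pack the CBP_IonaV2 player's respawn location and rotation into save data.
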(event EventBeginPlay)

(event Collision|EventActorBeginOverlap
  (params (OtherActor :type Actor%20Object%20Reference)))

(event EventTick
  (params (DeltaSeconds :type Float%20%28single-precision%29)))

(event EventSyncAfterLoad
  (params (InData :type Save%20Data%20Structure%20%28by%20ref%29)))

(fn ConstructionScript)

(fn SyncBeforeSave)