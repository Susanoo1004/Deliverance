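; Checkpoint actor that records a respawn point and saves the game when the CBP_IonaV2 character overlaps it.
; The character's respawn location comes from RespawnDummy and its rotation from CameraShadow, then the SaveSystem on CustomGameInstance saves asynchronously.
; The construction script applies Color and Opacity to the materials of both helpers and TriggerBoxVisual.
; An asynchronous load call is present but never runs.
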(event EventBeginPlay)

(event Collision|EventActorBeginOverlap
  (params (OtherActor :type Actor%20Object%20Reference))
  (bind _ascbp_iona_v2 (Utilities|Casting|CastToCBP_IonaV2 OtherActor))
  (Variables|/Game/DrownedPath/Entities/Player/BP/Character/CBP_IonaV2.CBP_IonaV2_C|SetRespawnLocation _ascbp_iona_v2 (Transformation|GetWorldLocation (Variables|Default|GetRespawnDummy)))
  (Variables|/Game/DrownedPath/Entities/Player/BP/Character/CBP_IonaV2.CBP_IonaV2_C|SetRespawnRotation _ascbp_iona_v2 (Transformation|GetWorldRotation (Variables|Default|GetCameraShadow)))
  (bind _ascustom_game_instance (Utilities|Casting|CastToCustomGameInstance (Game|GetGameInstance)))
  (Class|SaveSystem|ASynchronousSaveGame (Variables|/Game/DrownedPath/Core/GameMode/CustomGameInstance.CustomGameInstance_C|GetSaveSystem _ascustom_game_instance)))

(event EventTick
  (params (DeltaSeconds :type Float%20%28single-precision%29)))

(fn ConstructionScript
  (Rendering|Material|SetVectorParameterValueonMaterials (Variables|Default|GetCameraShadow) "Color" (Math|Conversions|ToVector(LinearColor) (Variables|Default|GetColor)))
  (Rendering|Material|SetScalarParameterValueonMaterials (Variables|Default|GetCameraShadow) "Opacity" (Variables|Default|GetOpacity))
  (Rendering|Material|SetVectorParameterValueonMaterials (Variables|Default|GetRespawnDummy) "Color" (Math|Conversions|ToVector(LinearColor) (Variables|Default|GetColor)))
  (Rendering|Material|SetScalarParameterValueonMaterials (Variables|Default|GetRespawnDummy) "Opacity" (Variables|Default|GetOpacity))
  (Rendering|Material|SetVectorParameterValueonMaterials (Variables|Default|GetTriggerBoxVisual) "Color" (Math|Conversions|ToVector(LinearColor) (Variables|Default|GetColor)))
  (Rendering|Material|SetScalarParameterValueonMaterials (Variables|Default|GetTriggerBoxVisual) "Opacity" (Variables|Default|GetOpacity)))